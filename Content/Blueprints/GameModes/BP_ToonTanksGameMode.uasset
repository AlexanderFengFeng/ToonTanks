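; Toon Tanks game mode Blueprint that shows the UI for the start and end of a match.
; The StartGame event creates the start game widget and adds it to the viewport.
; The GameOver event adds the game over widget, using its WonGame flag to show a green congratulations message or a red game over message.
; BeginPlay, Tick and the construction script contain no logic.
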(event EventBeginPlay)

(event EventTick
  (params (DeltaSeconds :type Float%20%28single-precision%29)))

(event EventStartGame
  (bind _returnvalue (UserInterface|CreateWidget "/Game/Blueprints/Widgets/WBP_StartGameWidget.WBP_StartGameWidget_C"))
  (UserInterface|Viewport|AddtoViewport _returnvalue 0))

(event EventGameOver
  (params (bWonGame :type Boolean))
  (bind _returnvalue (UserInterface|CreateWidget "/Game/Blueprints/Widgets/WBP_GameOverWidget.WBP_GameOverWidget_C"))
  (UserInterface|Viewport|AddtoViewport _returnvalue 0)
  (Rendering|Components|TextRender|SetText (Variables|/Game/Blueprints/Widgets/WBP_GameOverWidget.WBP_GameOverWidget_C|GetDisplayText _returnvalue) (select bWonGame "Congratulations!" "Game Over!"))
  (Appearance|SetColorandOpacity (Variables|/Game/Blueprints/Widgets/WBP_GameOverWidget.WBP_GameOverWidget_C|GetDisplayText _returnvalue) (select bWonGame (Utilities|Struct|MakeSlateColor "(R=0.000000,G=1.000000,B=0.227451,A=1.000000)") (Utilities|Struct|MakeSlateColor "(R=0.953125,G=0.034479,B=0.004964,A=1.000000)")) :!class /Script/UMG.TextBlock))

(fn ConstructionScript)