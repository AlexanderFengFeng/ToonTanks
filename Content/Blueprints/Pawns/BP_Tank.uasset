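; BP_Tank is a tank pawn Blueprint that drives the player's on-screen health display.
; On BeginPlay it creates WBP_HUDWidget for player controller 0, adds it to the viewport and starts the displayed health at full.
; Each Tick, while Health's percentage is below the displayed value, it lowers that value at VisualHealthChangeRate and pushes it to the widget, animating damage as a gradual drain.
; Health increases are not reflected.
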(event EventBeginPlay
  (bind _returnvalue (UserInterface|CreateWidget "/Game/Blueprints/Widgets/WBP_HUDWidget.WBP_HUDWidget_C" (Game|GetPlayerController 0)))
  (bind _output_get (Variables|Default|SetHUDWidget _returnvalue))
  (UserInterface|Viewport|AddtoViewport _output_get 0)
  (Variables|Default|SetLastRecordedHealthPercent 1.0))

(event Collision|EventActorBeginOverlap
  (params (OtherActor :type Actor%20Object%20Reference)))

(event EventTick
  (params (DeltaSeconds :type Float%20%28single-precision%29))
  (if (< (Class|HealthComponent|GetHealthPercentage (Variables|Default|GetHealth)) (Variables|Default|GetLastRecordedHealthPercent))
    (Default|SetPercent (Variables|Default|GetHUDWidget) (- (Variables|Default|GetLastRecordedHealthPercent) (* DeltaSeconds (Variables|Default|GetVisualHealthChangeRate))))
    (Variables|Default|SetLastRecordedHealthPercent (- (Variables|Default|GetLastRecordedHealthPercent) (* DeltaSeconds (Variables|Default|GetVisualHealthChangeRate))))))

(fn ConstructionScript)